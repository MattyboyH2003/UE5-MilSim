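; BP_DriverSeat is the driver's seat of a vehicle, a possessable seat that turns player input into driving commands.
; Its GetInSeat and GetOutSeat overrides call the parent logic and add or remove the IMC_Driver Enhanced Input mapping context.
; Throttle, turn and brake input actions cast the parent actor to BP_VehicleBase and forward their values to it.
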(event Input|EnhancedActionEvents|EnhancedInputActionIA_Throttle
  (params (ActionValue :type Float%20%28double-precision%29) (ElapsedSeconds :type Float%20%28double-precision%29) (TriggeredSeconds :type Float%20%28double-precision%29) (InputAction :type Input%20Action%20Object%20Reference :default "/Game/Player/Input/Vehicles/IA_Throttle.IA_Throttle"))
  ;[1 1 1] Throttle
  (:Triggered
    (bind _asbp_vehicle_base (Utilities|Casting|CastToBP_VehicleBase (Actor|GetParentActor)))
    (Default|ApplyThrottle _asbp_vehicle_base ActionValue)))

(event Input|EnhancedActionEvents|EnhancedInputActionIA_Turn
  (params (ActionValue :type Float%20%28double-precision%29) (ElapsedSeconds :type Float%20%28double-precision%29) (TriggeredSeconds :type Float%20%28double-precision%29) (InputAction :type Input%20Action%20Object%20Reference :default "/Game/Player/Input/Vehicles/IA_Turn.IA_Turn"))
  ;[1 1 1] Turning
  (:Triggered
    (bind _asbp_vehicle_base (Utilities|Casting|CastToBP_VehicleBase (Actor|GetParentActor)))
    (Default|Turn _asbp_vehicle_base ActionValue)))

(event Input|EnhancedActionEvents|EnhancedInputActionIA_Brake
  (params (ActionValue :type Float%20%28double-precision%29) (ElapsedSeconds :type Float%20%28double-precision%29) (TriggeredSeconds :type Float%20%28double-precision%29) (InputAction :type Input%20Action%20Object%20Reference :default "/Game/Player/Input/Vehicles/IA_Brake.IA_Brake"))
  ;[1 1 1] Brake
  (:Triggered
    (bind _asbp_vehicle_base (Utilities|Casting|CastToBP_VehicleBase (Actor|GetParentActor)))
    (Default|ApplyBrake _asbp_vehicle_base ActionValue)))

(fn ConstructionScript)

(fn GetinSeat
  (params (Player :type BP%20Player%20Character%20Object%20Reference))
  (|CallParentFunction Player)
  ;[1 1 1] Enhanced Input Component
  (bind _asplayer_controller (Utilities|Casting|CastToPlayerController (Pawn|GetController)))
  (Utilities|IsValid (PlayerController|LocalPlayerSubsystems|GetEnhancedInputLocalPlayerSubsystem _asplayer_controller)
    (:Is%20Valid
      (Input|AddMappingContext (PlayerController|LocalPlayerSubsystems|GetEnhancedInputLocalPlayerSubsystem _asplayer_controller) "/Game/Player/Input/Vehicles/IMC_Driver.IMC_Driver" 0 "(bIgnoreAllPressedKeysUntilRelease=True,bForceImmediately=False)"))))

(fn GetOutSeat
  (bind _asplayer_controller (Utilities|Casting|CastToPlayerController (Pawn|GetController)))
  (Input|RemoveMappingContext (PlayerController|LocalPlayerSubsystems|GetEnhancedInputLocalPlayerSubsystem _asplayer_controller) "/Game/Player/Input/Vehicles/IMC_Driver.IMC_Driver" "(bIgnoreAllPressedKeysUntilRelease=True,bForceImmediately=False)")
  (|CallParentFunction))