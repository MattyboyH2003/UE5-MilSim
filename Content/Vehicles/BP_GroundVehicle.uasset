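; BP_GroundVehicle is a ground vehicle Blueprint that tracks speed through throttle and brake events.
; ApplyThrottle adds a scaled input amount to the Velocity variable, and ApplyBrake subtracts one, with no clamping or delta-time scaling.
; Both events print the new value for debugging, and the graphs shown never use Velocity to move the vehicle.
; The construction script only calls its parent.
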(event EventApplyBrake
  (params (BrakeAmount :type Float%20%28double-precision%29))
  (bind _output_get (Variables|Default|SetVelocity (- (Variables|Default|GetVelocity) (* BrakeAmount 1e+01))))
  (Development|PrintString (Class|KismetStringLibrary|BuildStringDouble "Velocity: " "" _output_get)))

(event EventApplyThrottle
  (params (ThrottleAmount :type Float%20%28double-precision%29))
  (bind _output_get (Variables|Default|SetVelocity (+ (Variables|Default|GetVelocity) (* ThrottleAmount 1e+01))))
  (Development|PrintString (Class|KismetStringLibrary|BuildStringDouble "Velocity: " "" _output_get)))

(fn ConstructionScript
  (|CallParentFunction))