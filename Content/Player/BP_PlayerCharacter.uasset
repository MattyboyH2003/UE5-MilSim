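; BP_PlayerCharacter is the player character, with Enhanced Input movement, look, jump and vehicle entry.
; BeginPlay adds the IMC_Player mapping context, whose actions drive movement and controller rotation.
; Interact runs a debug-drawn Visibility trace from the camera and, on hitting a BP_West_Truck_M983HEMTT, gets its driver seat.
; The character registers as that seat's driver, snaps onto it, and the player controller possesses the seat.
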(event Input|EnhancedActionEvents|EnhancedInputActionIA_Look
  (params (ActionValue :type Vector%202D%20Structure) (ElapsedSeconds :type Float%20%28double-precision%29) (TriggeredSeconds :type Float%20%28double-precision%29) (InputAction :type Input%20Action%20Object%20Reference :default "/Game/Player/Input/Player/IA_Look.IA_Look"))
  (:Triggered
    (Pawn|Input|AddControllerYawInput (.x ActionValue))
    (Pawn|Input|AddControllerPitchInput (.y ActionValue))))

(event Input|EnhancedActionEvents|EnhancedInputActionIA_Interact
  (params (ActionValue :type Boolean) (ElapsedSeconds :type Float%20%28double-precision%29) (TriggeredSeconds :type Float%20%28double-precision%29) (InputAction :type Input%20Action%20Object%20Reference :default "/Game/Player/Input/Player/IA_Interact.IA_Interact"))
  (bind _camera (Variables|Default|GetCamera))
  (bind _returnvalue (Transformation|GetWorldLocation _camera))
  (:Triggered
    ;[1 1 1] Line Tracing
    (bind _outhit (Collision|LineTraceByChannel _returnvalue (+ _returnvalue (* (Math|Vector|GetForwardVector _camera) 10000)) "TraceTypeQuery1" false 0 "ForOneFrame"))
    ;[1 1 1] Get Driver Seat
    (if (Utilities|ClassIsChildOf (Utilities|GetClass (.hitactor _outhit)) "/Game/VigilanteContent/Vehicles/West_Truck_M983HEMTT/BP_West_Truck_M983HEMTT.BP_West_Truck_M983HEMTT_C")
      (bind _asbp_west_truck_m983hemtt (Utilities|Casting|CastToBP_West_Truck_M983HEMTT (.hitactor _outhit)))
      (bind _driver_seat_pawn (Default|GetDriverSeat _asbp_west_truck_m983hemtt))
      ;[1 1 1] Possess
      (Default|SetDriver _driver_seat_pawn self)
      (Transformation|AttachActorToActor _driver_seat_pawn "None" "SnapToTarget" "SnapToTarget" "SnapToTarget" true)
      (Pawn|Possess (Game|GetPlayerController 0) _driver_seat_pawn))))

(event Input|EnhancedActionEvents|EnhancedInputActionIA_Jump
  (params (ActionValue :type Boolean) (ElapsedSeconds :type Float%20%28double-precision%29) (TriggeredSeconds :type Float%20%28double-precision%29) (InputAction :type Input%20Action%20Object%20Reference :default "/Game/Player/Input/Player/IA_Jump.IA_Jump"))
  (:Triggered
    (Character|Jump)))

(event Input|EnhancedActionEvents|EnhancedInputActionIA_Move
  (params (ActionValue :type Vector%202D%20Structure) (ElapsedSeconds :type Float%20%28double-precision%29) (TriggeredSeconds :type Float%20%28double-precision%29) (InputAction :type Input%20Action%20Object%20Reference :default "/Game/Player/Input/Player/IA_Move.IA_Move"))
  (:Triggered
    (Pawn|Input|AddMovementInput (Transformation|GetActorRightVector) (.x ActionValue) false)
    (Pawn|Input|AddMovementInput (Transformation|GetActorForwardVector) (.y ActionValue) false)))

(event EventBeginPlay
  (bind _returnvalue (Game|GetPlayerController 0))
  (bind _returnvalue_2 (PlayerController|LocalPlayerSubsystems|GetEnhancedInputLocalPlayerSubsystem _returnvalue))
  (Utilities|IsValid _returnvalue_2
    (:Is%20Valid
      (Input|AddMappingContext _returnvalue_2 "/Game/Player/Input/Player/IMC_Player.IMC_Player" 0 "(bIgnoreAllPressedKeysUntilRelease=True,bForceImmediately=False)"))))

(event Collision|EventActorBeginOverlap
  (params (OtherActor :type Actor%20Object%20Reference)))

(event EventTick
  (params (DeltaSeconds :type Float%20%28single-precision%29)))

(fn ConstructionScript)