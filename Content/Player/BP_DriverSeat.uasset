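; BP_DriverSeat is a player-possessable seat that lets the stored driver get out and regain control.
; On BeginPlay it adds the IMC_Driver Enhanced Input mapping context to the first local player.
; SetDriver stores the occupant as Driver.
; Pressing IA_Interact detaches that Driver, keeping its world transform, and has player controller 0 possess it again; entering the seat is not handled here.
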(event Input|EnhancedActionEvents|EnhancedInputActionIA_Interact
  (params (ActionValue :type Boolean) (ElapsedSeconds :type Float%20%28double-precision%29) (TriggeredSeconds :type Float%20%28double-precision%29) (InputAction :type Input%20Action%20Object%20Reference :default "/Game/Player/Input/Player/IA_Interact.IA_Interact"))
  (bind _driver (Variables|Default|GetDriver))
  (:Started
    (Transformation|DetachFromActor _driver "KeepWorld" "KeepWorld" "KeepWorld")
    (Pawn|Possess (Game|GetPlayerController 0) _driver)))

(event EventBeginPlay
  (bind _returnvalue (Game|GetPlayerController 0))
  (bind _returnvalue_2 (PlayerController|LocalPlayerSubsystems|GetEnhancedInputLocalPlayerSubsystem _returnvalue))
  (Utilities|IsValid _returnvalue_2
    (:Is%20Valid
      (Input|AddMappingContext _returnvalue_2 "/Game/Player/Input/Driving/IMC_Driver.IMC_Driver" 0 "(bIgnoreAllPressedKeysUntilRelease=True,bForceImmediately=False)"))))

(event Collision|EventActorBeginOverlap
  (params (OtherActor :type Actor%20Object%20Reference)))

(event EventTick
  (params (DeltaSeconds :type Float%20%28single-precision%29)))

(fn ConstructionScript)

(fn SetDriver
  (params (Player :type BP%20Player%20Character%20Object%20Reference))
  (Variables|Default|SetDriver Player))